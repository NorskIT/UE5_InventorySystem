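; Master item actor for the inventory system, representing a pickup in the world.
; LookAt reads the item's row from the data table referenced by its BPCItemData component and returns a "Pick up" prompt with the E key plus a description.
; RemoveItem destroys the actor, and the Destroyed event adds it to the ActorsRemoved list in the third-person game mode's level save data.
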(event EventDestroyed
  (bind _asbp_third_person_game_mode (Utilities|Casting|CastToBP_ThirdPersonGameMode (Game|GetGameMode)))
  (Utilities|Array|AddUnique (Variables|/Game/Game/InventorySystem/BP_SaveData_Level.BP_SaveData_Level_C|GetActorsRemoved (Variables|/Game/Game/ThirdPerson/Blueprints/BP_ThirdPersonGameMode.BP_ThirdPersonGameMode_C|GetSave%20Data%20Level _asbp_third_person_game_mode)) (Utilities|ResolveSoftReference self)))

(fn ConstructionScript)

(fn RemoveItem
  (Actor|DestroyActor))

(fn Lookat
  (bind _bpc_itemdata (Variables|Default|GetBPC_ItemData))
  (bind _itemid (Variables|/Game/Game/InventorySystem/BPC_ItemData.BPC_ItemData_C|GetItemId _bpc_itemdata))
  (bind _returnvalue (Utilities|GetDataTableRow (.datatable _itemid) (.rowname _itemid))
    (:then
      (return (Utilities|Text|ToText(String) (Utilities|String|Append "Pick up " (Utilities|String|ToString(Text) (.Name (Utilities|Struct|BreakFItemStruct _returnvalue))) " (E)")) (.Description (Utilities|Struct|BreakFItemStruct _returnvalue))))))