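; BPC_ItemData is an actor component that makes its owning actor a pickup item for the inventory system.
; It turns on replication for the owner at BeginPlay.
; On interaction it adds its item row ID and quantity to the player's inventory component and destroys the owner if that succeeds.
; Its LookAt function currently returns an empty message and description.
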(event EventBeginPlay
  (Networking|SetReplicates (Components|GetOwner) true))

(event EventInteractwith
  (params (PlayerCharacter :type BP%20Player%20Character%20Object%20Reference))
  (bind _bpc_inventory (Variables|/Game/Game/Player/BP_PlayerCharacter.BP_PlayerCharacter_C|GetBPC_Inventory PlayerCharacter))
  (Utilities|IsValid _bpc_inventory
    (:Is%20Valid
      (bind _sucess (Default|AddtoInventory _bpc_inventory (.rowname (Variables|Default|GetItemId)) (Variables|Default|GetQuantity)))
      (if _sucess
        (Actor|DestroyActor (Components|GetOwner))))))

(fn Lookat
  (return "" ""))