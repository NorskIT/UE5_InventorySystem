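; BP_M_Container is an interactable world container that holds items in an inventory component.
; Interacting with it tells the player character's custom HUD to show that container's inventory.
; Its LookAt function supplies the container name and a count of the items inside as display text.
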(event EventInteractwith
  (params (PlayerCharacter :type BP%20Player%20Character%20Object%20Reference))
  (Default|ShowContainer (Variables|/Game/Game/Player/BP_PlayerCharacter.BP_PlayerCharacter_C|GetCustomHUD PlayerCharacter) (Variables|Default|GetBPC_Inventory)))

(fn ConstructionScript)

(fn Lookat
  (bind _amount (Default|GetAmountItemsinInventory (Variables|Default|GetBPC_Inventory)))
  (return (Utilities|Text|ToText(String) (Variables|Default|GetContainerName)) (Utilities|Text|ToText(String) (Utilities|String|Append (Utilities|String|ToString(Integer) _amount) " items inside"))))